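; Editor manager for the Building Hider system that previews and prepares buildings inside its box bounds for floor and directional hiding.
; Actor tags store hide directions and floor, driving visibility previews and a custom-depth stencil debug view.
; MergeToSingleMesh spawns mesh copies with tags and yaw packed into vertex colors, returning them with merge options.
; It also records collision volumes and selected actor classes into BuildingData.
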(event Custom|Set%20Vertex%20Color
  (CallFunction|SetActorsVertexColor))

(event Custom|Clear%20Vertex%20Color
  (CallFunction|ClearMeshVertexColor))

(event Custom|Update%20Visibility
  (CallFunction|UpdateActorsVisibility))

(fn ConstructionScript
  (bind _returnvalue (Transformation|GetActorLocation))
  (bind _returnvalue_2 (Transformation|GetActorScale3D))
  (bind _box (Variables|Default|GetBox))
  (bind (_x _y) (Math|Vector|BreakVector _returnvalue))
  (bind _boxextent (Variables|/Script/Engine.BoxComponent|GetBoxExtent _box))
  (bind _returnvalue_3 (* _boxextent 2.0))
  (bind _returnvalue_4 (* _returnvalue_3 _returnvalue_2))
  (bind (_x_2 _y_2 _z) (Math|Vector|BreakVector _returnvalue_4))
  (Variables|Default|SetActiveFloor (Math|Integer|Clamp(Integer) (Variables|Default|GetActiveFloor) 0 99))
  (Transformation|SetActorRotation "0, 0, 0")
  (Transformation|SetActorLocation (Math|Vector|MakeVector _x _y 1e+01) false false)
  (Rendering|Material|SetVectorParameterValue 0 "/Game/Building_Hider/Material_Functions/MPC_BuildingHider.MPC_BuildingHider" "TargetLocation" (Math|Color|MakeColor 1e+04 1e+04 -1e+04 0.0) :!class /Script/Engine.KismetMaterialLibrary)
  (bind _asbp_border (Utilities|Casting|CastToBP_Border (Variables|/Script/Engine.ChildActorComponent|GetChildActor (Variables|Default|GetBorder))))
  (Variables|/Game/Building_Hider/Demo/Blueprints/Border/BP_Border.BP_Border_C|SetBorderSIze _asbp_border (Math|Vector2D|MakeVector2D _x_2 _y_2))
  (Variables|/Game/Building_Hider/Demo/Blueprints/Border/BP_Border.BP_Border_C|SetBorderHeight _asbp_border _z)
  (Default|SetupBorder _asbp_border))

(fn GetActorsinBounds
  (bind _returnvalue (Transformation|GetActorScale3D))
  (bind _returnvalue_2 (Transformation|GetActorLocation))
  (bind _box (Variables|Default|GetBox))
  (bind (_x _y _z) (Math|Vector|BreakVector _returnvalue_2))
  (bind _boxextent (Variables|/Script/Engine.BoxComponent|GetBoxExtent _box))
  (bind _returnvalue_3 (* _boxextent _returnvalue))
  (bind (_x_2 _y_2 _z_2) (Math|Vector|BreakVector _returnvalue_3))
  (bind _outactors (Actor|GetAllActorsOfClass 0 "/Script/Engine.Actor"))
  (for _array_element _outactors
    (if (Math|Boolean|ANDBoolean (< (.X (Math|Vector|BreakVector (Transformation|GetActorLocation _array_element))) (+ _x _x_2)) (> (.X (Math|Vector|BreakVector (Transformation|GetActorLocation _array_element))) (- _x _x_2)) (< (.Y (Math|Vector|BreakVector (Transformation|GetActorLocation _array_element))) (+ _y _y_2)) (> (.Y (Math|Vector|BreakVector (Transformation|GetActorLocation _array_element))) (- _y _y_2)) (< (.Z (Math|Vector|BreakVector (Transformation|GetActorLocation _array_element))) (+ _z _z_2)) (> (.Z (Math|Vector|BreakVector (Transformation|GetActorLocation _array_element))) (- _z _z_2)))
      (if (and (!= (Utilities|GetClass _array_element) "UBP_BH_Editor_Manager_C") (!= (Utilities|GetClass _array_element) "/Script/NavigationSystem.RecastNavMesh"))
        (Utilities|Array|Add (LocalVariables|GetActorsLOCAL) _array_element))))
  (return (LocalVariables|GetActorsLOCAL)))

(fn UpdateActorsVisibility
  (bind _outactors (Actor|GetAllActorsOfClass 0 "/Game/Building_Hider/Blueprints/Collisions/Parent_Class/UBP_BH_Collision.UBP_BH_Collision_C"))
  (for _array_element _outactors
    (Rendering|SetVisibility (Variables|/Script/Engine.Actor|GetRootComponent _array_element) (and (>= (Variables|Default|GetActiveFloor) (Default|GetFloorNum _array_element)) (not (Variables|Default|GetHideCollisionsEnabled))) true))
  (bind _actors (CallFunction|GetActorsinBounds))
  (for _array_element_2 _actors
    (LocalVariables|SetActorLOCAL _array_element_2)
    (if (not (Utilities|ClassIsChildOf (Utilities|GetClass (LocalVariables|GetActorLOCAL)) "/Game/Building_Hider/Blueprints/Collisions/Parent_Class/UBP_BH_Collision.UBP_BH_Collision_C"))
      (LocalVariables|SetCurrentFloorLOCAL (CallFunction|CheckActorTag (LocalVariables|GetActorLOCAL) 4))
      (CallFunction|ShowDebugView (LocalVariables|GetActorLOCAL))
      (if (>= (Variables|Default|GetActiveFloor) (LocalVariables|GetCurrentFloorLOCAL))
        (Rendering|SetVisibility (Variables|/Script/Engine.Actor|GetRootComponent (LocalVariables|GetActorLOCAL)) true true)
        (if (Variables|Default|GetHideForAllFloors)
          (Utilities|FlowControl|Sequence :!label _label
            (:then_0
              (if (Variables|Default|GetHideDir1)
                (if (== (CallFunction|CheckActorTag (LocalVariables|GetActorLOCAL)) 1)
                  (Rendering|SetVisibility (Variables|/Script/Engine.Actor|GetRootComponent (LocalVariables|GetActorLOCAL)) false true))))
            (:then_1
              (if (Variables|Default|GetHideDir2)
                (if (== (CallFunction|CheckActorTag (LocalVariables|GetActorLOCAL) 1) 1)
                  (Rendering|SetVisibility (Variables|/Script/Engine.Actor|GetRootComponent (LocalVariables|GetActorLOCAL)) false true))))
            (:then_2
              (if (Variables|Default|GetHideDir3)
                (if (== (CallFunction|CheckActorTag (LocalVariables|GetActorLOCAL) 2) 1)
                  (Rendering|SetVisibility (Variables|/Script/Engine.Actor|GetRootComponent (LocalVariables|GetActorLOCAL)) false true))))
            (:then_3
              (if (Variables|Default|GetHideDir4)
                (if (== (CallFunction|CheckActorTag (LocalVariables|GetActorLOCAL) 3) 1)
                  (Rendering|SetVisibility (Variables|/Script/Engine.Actor|GetRootComponent (LocalVariables|GetActorLOCAL)) false true)))))
          (elif (== (Variables|Default|GetActiveFloor) (LocalVariables|GetCurrentFloorLOCAL))
            (goto _label)))
        (else
          (Rendering|SetVisibility (Variables|/Script/Engine.Actor|GetRootComponent (LocalVariables|GetActorLOCAL)) false true))))))

(fn MergetoSingleMesh
  (bind _meshname (Variables|Default|GetMeshName))
  (LocalVariables|SetLengthLOCAL (Utilities|Array|Length (Variables|Default|GetActorsForCollectingData)))
  (bind _actors (CallFunction|GetActorsinBounds))
  (for _array_element _actors
    (LocalVariables|SetActorLOCAL _array_element)
    (CallFunction|TagFiltering (LocalVariables|GetActorLOCAL))
    (bind _asstatic_mesh_actor (Utilities|Casting|CastToStaticMeshActor (LocalVariables|GetActorLOCAL))
      (:then
        (bind _returnvalue (Game|SpawnActorfromClass 0 "/Script/Engine.StaticMeshActor" (Transformation|GetActorTransform _asstatic_mesh_actor) "AlwaysSpawn" 0 0))
        (Components|StaticMesh|SetStaticMesh (Variables|/Script/Engine.StaticMeshActor|GetStaticMeshComponent _returnvalue) (Variables|/Script/Engine.StaticMeshComponent|GetStaticMesh (Variables|/Script/Engine.StaticMeshActor|GetStaticMeshComponent _asstatic_mesh_actor)))
        (Utilities|Array|Add (LocalVariables|GetActorsForMergeLOCAL) _returnvalue)
        (Class|MeshVertexPainterKismetLibrary|PaintVerticesSingleColor (Variables|/Script/Engine.StaticMeshActor|GetStaticMeshComponent _returnvalue) (Math|Color|MakeColor (+ (/ (Math|Float|SelectFloat 0.0 (Math|Float|SelectFloat 1.0 (Math|Float|SelectFloat 2.0 3.0 (and (<= (Math|Conversions|ToFloat(Integer) (Utilities|String|ToString(Name) (Utilities|Array|Get(acopy) (Variables|/Script/Engine.Actor|GetTags (LocalVariables|GetActorLOCAL)) 3))) 0.0) (>= (Math|Conversions|ToFloat(Integer) (Utilities|String|ToString(Name) (Utilities|Array|Get(acopy) (Variables|/Script/Engine.Actor|GetTags (LocalVariables|GetActorLOCAL)) 2))) 1.0))) (and (>= (Math|Conversions|ToFloat(Integer) (Utilities|String|ToString(Name) (Utilities|Array|Get(acopy) (Variables|/Script/Engine.Actor|GetTags (LocalVariables|GetActorLOCAL)) 3))) 1.0) (<= (Math|Conversions|ToFloat(Integer) (Utilities|String|ToString(Name) (Utilities|Array|Get(acopy) (Variables|/Script/Engine.Actor|GetTags (LocalVariables|GetActorLOCAL)) 2))) 0.0))) (and (<= (Math|Conversions|ToFloat(Integer) (Utilities|String|ToString(Name) (Utilities|Array|Get(acopy) (Variables|/Script/Engine.Actor|GetTags (LocalVariables|GetActorLOCAL)) 3))) 0.0) (<= (Math|Conversions|ToFloat(Integer) (Utilities|String|ToString(Name) (Utilities|Array|Get(acopy) (Variables|/Script/Engine.Actor|GetTags (LocalVariables|GetActorLOCAL)) 2))) 0.0))) 1e+01) (/ (Math|Float|SelectFloat 0.0 (Math|Float|SelectFloat 1.0 (Math|Float|SelectFloat 2.0 3.0 (and (<= (Math|Conversions|ToFloat(Integer) (Utilities|String|ToString(Name) (Utilities|Array|Get(acopy) (Variables|/Script/Engine.Actor|GetTags (LocalVariables|GetActorLOCAL))))) 0.0) (>= (Math|Conversions|ToFloat(Integer) (Utilities|String|ToString(Name) (Utilities|Array|Get(acopy) (Variables|/Script/Engine.Actor|GetTags (LocalVariables|GetActorLOCAL)) 1))) 1.0))) (and (>= (Math|Conversions|ToFloat(Integer) (Utilities|String|ToString(Name) (Utilities|Array|Get(acopy) (Variables|/Script/Engine.Actor|GetTags (LocalVariables|GetActorLOCAL))))) 1.0) (<= (Math|Conversions|ToFloat(Integer) (Utilities|String|ToString(Name) (Utilities|Array|Get(acopy) (Variables|/Script/Engine.Actor|GetTags (LocalVariables|GetActorLOCAL)) 1))) 0.0))) (and (<= (Math|Conversions|ToFloat(Integer) (Utilities|String|ToString(Name) (Utilities|Array|Get(acopy) (Variables|/Script/Engine.Actor|GetTags (LocalVariables|GetActorLOCAL))))) 0.0) (<= (Math|Conversions|ToFloat(Integer) (Utilities|String|ToString(Name) (Utilities|Array|Get(acopy) (Variables|/Script/Engine.Actor|GetTags (LocalVariables|GetActorLOCAL)) 1))) 0.0))) 1e+02)) (Math|Float|Absolute(Float) (- 1.0 (/ (Class|KismetMathLibrary|ClampAxis (.Yaw (Math|Rotator|BreakRotator (Transformation|GetActorRotation _asstatic_mesh_actor)))) 3.6e+02))) (/ (Math|Conversions|ToFloat(Integer) (Utilities|String|ToString(Name) (Utilities|Array|Get(acopy) (Variables|/Script/Engine.Actor|GetTags (LocalVariables|GetActorLOCAL)) 4))) 1e+02) (Math|Float|SelectFloat 0.0 1.0 (< (Math|Conversions|ToFloat(Integer) (Utilities|String|ToString(Name) (Utilities|Array|Get(acopy) (Variables|/Script/Engine.Actor|GetTags (LocalVariables|GetActorLOCAL)) 5))) 1.0))) false)
        (for (_array_element_2 _array_index) (Rendering|Material|GetMaterials (Variables|/Script/Engine.StaticMeshActor|GetStaticMeshComponent _asstatic_mesh_actor))
          (Rendering|Material|SetMaterial (Variables|/Script/Engine.StaticMeshActor|GetStaticMeshComponent _returnvalue) _array_index _array_element_2)))
      (:CastFailed
        (bind _asubp_bh_collision (Utilities|Casting|CastToUBP_BH_Collision (LocalVariables|GetActorLOCAL))
          (:then
            (Utilities|Array|Add (LocalVariables|GetCollisionDataLOCAL) (Utilities|Struct|MakeS_BH_CollisionData (Default|GetFloorNum _asubp_bh_collision) (Variables|/Game/Building_Hider/Blueprints/Collisions/Parent_Class/UBP_BH_Collision.UBP_BH_Collision_C|GetCollisionType _asubp_bh_collision) (Math|Vector|SelectVector (Math|Vector|MakeVector 0.0 0.0 (.Z (Math|Vector|BreakVector (Transformation|GetActorLocation _asubp_bh_collision)))) (+ (Transformation|GetActorLocation _asubp_bh_collision) (Math|Vector|MakeVector 0.0 0.0 (* 5e+01 (.Z (Math|Vector|BreakVector (Transformation|GetActorScale3D _asubp_bh_collision)))))) (== (Variables|/Game/Building_Hider/Blueprints/Collisions/Parent_Class/UBP_BH_Collision.UBP_BH_Collision_C|GetCollisionType _asubp_bh_collision) 2)) (Transformation|GetActorRotation _asubp_bh_collision) (* "50.000000,50.000000,50.000000" (Transformation|GetActorScale3D _asubp_bh_collision)))))
          (:CastFailed
            (if (> (LocalVariables|GetLengthLOCAL) 0)
              (if (>= (Utilities|Array|FindItem (Variables|Default|GetActorsForCollectingData) (Utilities|GetClass (LocalVariables|GetActorLOCAL))) 0)
                (Utilities|Array|Add (LocalVariables|GetActorsLOCAL) (Utilities|Struct|MakeS_BH_ActorData (Utilities|GetClass (LocalVariables|GetActorLOCAL)) (Transformation|GetActorTransform (LocalVariables|GetActorLOCAL)) (Math|Conversions|ToInteger(Byte) (Utilities|String|ToString(Name) (Utilities|Array|Get(acopy) (Variables|/Script/Engine.Actor|GetTags (LocalVariables|GetActorLOCAL)) 4))) (Math|Integer|SelectInt 0 1 (== (Math|Conversions|ToInteger(Byte) (Utilities|String|ToString(Name) (Utilities|Array|Get(acopy) (Variables|/Script/Engine.Actor|GetTags (LocalVariables|GetActorLOCAL)) 1))) 0)) (Math|Integer|SelectInt 0 2 (== (Math|Conversions|ToInteger(Byte) (Utilities|String|ToString(Name) (Utilities|Array|Get(acopy) (Variables|/Script/Engine.Actor|GetTags (LocalVariables|GetActorLOCAL))))) 0)) (Math|Integer|SelectInt 0 3 (== (Math|Conversions|ToInteger(Byte) (Utilities|String|ToString(Name) (Utilities|Array|Get(acopy) (Variables|/Script/Engine.Actor|GetTags (LocalVariables|GetActorLOCAL)) 2))) 0)) (Math|Integer|SelectInt 0 4 (== (Math|Conversions|ToInteger(Byte) (Utilities|String|ToString(Name) (Utilities|Array|Get(acopy) (Variables|/Script/Engine.Actor|GetTags (LocalVariables|GetActorLOCAL)) 3))) 0)))))))))))
  (Utilities|Struct|SetmembersinMergeStaticMeshActorsOptions (Variables|Default|GetMergeOptions) (Utilities|String|Append (Variables|Default|GetMeshSavePath) "/" _meshname) _meshname)
  (Variables|Default|SetBuildingData (Utilities|Struct|MakeS_BH_BuildingData (LocalVariables|GetCollisionDataLOCAL) (LocalVariables|GetActorsLOCAL)))
  (return (LocalVariables|GetActorsForMergeLOCAL) (Variables|Default|GetMergeOptions)))

(fn ClearMeshVertexColor
  (bind _actors (CallFunction|GetActorsinBounds))
  (for _array_element _actors
    (bind _asstatic_mesh_actor (Utilities|Casting|CastToStaticMeshActor _array_element))
    (Class|MeshVertexPainterKismetLibrary|PaintVerticesSingleColor (Variables|/Script/Engine.StaticMeshActor|GetStaticMeshComponent _asstatic_mesh_actor) (Math|Color|MakeColor 1.0 1.0 1.0) true)))

(fn SetActorsVertexColor
  (bind _actors (CallFunction|GetActorsinBounds))
  (for _array_element _actors
    (LocalVariables|SetTagsLOCAL (Variables|/Script/Engine.Actor|GetTags _array_element))
    (Utilities|FlowControl|Sequence
      (:then_0
        (Utilities|FlowControl|Sequence
          (:then_0
            (if (not (Utilities|Array|IsValidIndex (LocalVariables|GetTagsLOCAL)))
              (Utilities|Array|SetArrayElem (LocalVariables|GetTagsLOCAL) 0 "0" true)))
          (:then_1
            (if (not (Utilities|Array|IsValidIndex (LocalVariables|GetTagsLOCAL) 1))
              (Utilities|Array|SetArrayElem (LocalVariables|GetTagsLOCAL) 1 "0" true)))
          (:then_2
            (if (not (Utilities|Array|IsValidIndex (LocalVariables|GetTagsLOCAL) 2))
              (Utilities|Array|SetArrayElem (LocalVariables|GetTagsLOCAL) 2 "0" true)))
          (:then_3
            (if (not (Utilities|Array|IsValidIndex (LocalVariables|GetTagsLOCAL) 3))
              (Utilities|Array|SetArrayElem (LocalVariables|GetTagsLOCAL) 3 "0" true)))
          (:then_4
            (if (not (Utilities|Array|IsValidIndex (LocalVariables|GetTagsLOCAL) 4))
              (Utilities|Array|SetArrayElem (LocalVariables|GetTagsLOCAL) 4 "0" true)))
          (:then_5
            (if (not (Utilities|Array|IsValidIndex (LocalVariables|GetTagsLOCAL) 5))
              (Utilities|Array|SetArrayElem (LocalVariables|GetTagsLOCAL) 5 "0" true)))))
      (:then_1
        (bind _asstatic_mesh_actor (Utilities|Casting|CastToStaticMeshActor _array_element))
        (Class|MeshVertexPainterKismetLibrary|PaintVerticesSingleColor (Variables|/Script/Engine.StaticMeshActor|GetStaticMeshComponent _asstatic_mesh_actor) (Math|Color|MakeColor (+ (/ (Math|Conversions|ToFloat(Integer) (Utilities|String|ToString(Name) (Utilities|Array|Get(acopy) (LocalVariables|GetTagsLOCAL)))) 1e+01) (/ (Math|Conversions|ToFloat(Integer) (Utilities|String|ToString(Name) (Utilities|Array|Get(acopy) (LocalVariables|GetTagsLOCAL) 1))) 1e+02)) (+ (/ (Math|Conversions|ToFloat(Integer) (Utilities|String|ToString(Name) (Utilities|Array|Get(acopy) (LocalVariables|GetTagsLOCAL) 2))) 1e+01) (/ (Math|Conversions|ToFloat(Integer) (Utilities|String|ToString(Name) (Utilities|Array|Get(acopy) (LocalVariables|GetTagsLOCAL) 3))) 1e+02)) 0.0 (/ (Math|Conversions|ToFloat(Integer) (Utilities|String|ToString(Name) (Utilities|Array|Get(acopy) (LocalVariables|GetTagsLOCAL) 5))) 1e+01)) false)))))

(fn UpdateActorsTags
  (params (Actors :type Array%20of%20Actor%20Object%20References))
  (bind _tagslocal (LocalVariables|GetTagsLOCAL))
  (for _array_element Actors
    (for _index (range 0 5)
      (if (Utilities|Array|IsValidIndex (Variables|/Script/Engine.Actor|GetTags _array_element) _index)
        (Utilities|Array|Add _tagslocal (Utilities|Array|Get(acopy) (Variables|/Script/Engine.Actor|GetTags _array_element) _index))
        (else
          (Utilities|Array|Add _tagslocal "0"))))
    (Variables|/Script/Engine.Actor|SetTags _array_element (LocalVariables|GetTagsLOCAL))))

(fn CheckActorTag
  (params (Actor :type Actor%20Object%20Reference) (TagNum :type Integer))
  (bind _tags (Variables|/Script/Engine.Actor|GetTags Actor))
  (bind _output (Utilities|Array|Get(acopy) _tags TagNum))
  (if (Utilities|Array|IsValidIndex _tags TagNum)
    (if (Utilities|Name|Equal(Name) _output "None")
      (return 0)
      (else
        (return (Math|Conversions|ToInteger(Byte) (Utilities|String|ToString(Name) _output)))))
    (else
      (return 0))))

(fn TagFiltering
  (params (Actor :type Actor%20Object%20Reference))
  (bind _tags (Variables|/Script/Engine.Actor|GetTags Actor))
  (for _index (range 0 5)
    (if (Utilities|Array|IsValidIndex _tags _index)
      (if (Utilities|Name|Equal(Name) (Utilities|Array|Get(acopy) _tags _index) "None")
        (|SetBy-RefVar (Utilities|Array|Get(acopy) _tags _index) "0"))
      (else
        (Utilities|Array|Add _tags "0")))))

(fn ShowDebugView
  (params (Actor :type Actor%20Object%20Reference))
  (LocalVariables|SetComponentsLOCAL (Actor|GetComponentsByClass Actor "/Script/Engine.StaticMeshComponent"))
  (if (Variables|Default|GetDebugViewEnabled)
    (LocalVariables|SetColorIndexLOCAL (+ (* (CallFunction|CheckActorTag Actor) 1) (* (CallFunction|CheckActorTag Actor 1) 2) (* (CallFunction|CheckActorTag Actor 2) 4) (* (CallFunction|CheckActorTag Actor 3) 8) 1))
    (for _array_element (LocalVariables|GetComponentsLOCAL)
      (Rendering|SetRenderCustomDepth _array_element true)
      (Rendering|SetCustomDepthStencilValue _array_element (LocalVariables|GetColorIndexLOCAL)))
    (else
      (for _array_element_2 (LocalVariables|GetComponentsLOCAL)
        (Rendering|SetRenderCustomDepth _array_element_2 false)
        (Rendering|SetCustomDepthStencilValue _array_element_2 0)))))