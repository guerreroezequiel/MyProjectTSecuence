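; Selection manager component for the Building Hider system that tracks the selected building, switches its visible floor and activates or deactivates its hiding.
; Auto-hide and player-floor selection find the building around the pawn with sphere overlaps, and changes are pushed to the building widget.
; It installs a highlight post-process material at start and writes pawn location plus an active-floor flag to a Material Parameter Collection every tick.
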(event Custom|Event%20Switch%20Floor%20Up
  (bind _selectedbuilding (Variables|Default|GetSelectedBuilding))
  (Utilities|IsValid _selectedbuilding
    (:Is%20Valid
      (Default|SwitchFloorUp _selectedbuilding)
      (Default|EventUpdateBuildingInfo (Variables|Default|GetBuildingWidget) (Variables|Default|GetSelectedBuilding))
      (if (Variables|Default|GetAutoHide)
        (Public|SetAutoHideMode false)))))

(event Custom|Event%20Switch%20Floor%20Down
  (bind _selectedbuilding (Variables|Default|GetSelectedBuilding))
  (Utilities|IsValid _selectedbuilding
    (:Is%20Valid
      (Default|SwitchFloorDown _selectedbuilding)
      (Default|EventUpdateBuildingInfo (Variables|Default|GetBuildingWidget) (Variables|Default|GetSelectedBuilding))
      (if (Variables|Default|GetAutoHide)
        (Public|SetAutoHideMode false)))))

(event EventBeginPlay
  ;[0 0.2956 0.7448 0.1 16] Set Post Process material for buildings highlight
  (bind _returnvalue (Actor|GetActorOfClass "/Script/Engine.PostProcessVolume"))
  (Utilities|IsValid _returnvalue
    (:Is%20Valid
      (Utilities|Struct|SetmembersinPostProcessSettings (Variables|/Script/Engine.PostProcessVolume|GetSettings _returnvalue) (Utilities|Struct|MakeWeightedBlendables (Utilities|Array|MakeArray (Utilities|Struct|MakeWeightedBlendable 1.0 "/Game/Building_Hider/Blueprints/PostProcess/M_BH_Select_PostProcess.M_BH_Select_PostProcess")))))))

(event EventTick
  (params (DeltaSeconds :type Float%20%28single-precision%29))
  (bind _selectedbuilding (Variables|Default|GetSelectedBuilding))
  ;[0 0.2956 0.7448 0.1 16] This node transfers the character’s coordinates to the material
  (Variables|Default|SetPlayerLocation (Transformation|GetActorLocation (Pawn|GetControlledPawn (Game|GetPlayerController (Variables|Default|GetPlayerIndex)))))
  (Utilities|IsValid _selectedbuilding
    (:Is%20Valid
      (Rendering|Material|SetVectorParameterValue "/Game/Building_Hider/Material_Functions/MPC_BuildingHider.MPC_BuildingHider" "TargetLocation" (Math|Color|MakeColor (.X (Math|Vector|BreakVector (Variables|Default|GetPlayerLocation))) (.Y (Math|Vector|BreakVector (Variables|Default|GetPlayerLocation))) (.Z (Math|Vector|BreakVector (Variables|Default|GetPlayerLocation))) (Math|Conversions|ToFloat(Boolean) (Default|OnActiveFloor? _selectedbuilding (Variables|Default|GetPlayerLocation)))) :!class /Script/Engine.KismetMaterialLibrary))
    (:Is%20Not%20Valid
      (Rendering|Material|SetVectorParameterValue "/Game/Building_Hider/Material_Functions/MPC_BuildingHider.MPC_BuildingHider" "TargetLocation" (Math|Color|MakeColor (.X (Math|Vector|BreakVector (Variables|Default|GetPlayerLocation))) (.Y (Math|Vector|BreakVector (Variables|Default|GetPlayerLocation))) (.Z (Math|Vector|BreakVector (Variables|Default|GetPlayerLocation))) 0.0) :!class /Script/Engine.KismetMaterialLibrary))))

(fn SelectBuilding
  (params (Building :type Actor%20Object%20Reference))
  (bind _buildingwidget (Variables|Default|GetBuildingWidget))
  (bind _asbp_building_master (Utilities|Casting|CastToBP_Building_Master Building))
  (LocalVariables|SetNewBuildingLOCAL _asbp_building_master)
  (Utilities|FlowControl|Sequence
    (:then_0
      (if (!= (Variables|Default|GetSelectedBuilding) (LocalVariables|GetNewBuildingLOCAL))
        (Utilities|IsValid (Variables|Default|GetSelectedBuilding)
          (:Is%20Valid
            (Default|DeactivateHidden (Variables|Default|GetSelectedBuilding) false)
            (if (Variables|Default|GetAutoHide)
              (bind _outactors (Collision|SphereOverlapActors (Transformation|GetActorLocation (Pawn|GetControlledPawn (Game|GetPlayerController (Variables|Default|GetPlayerIndex)))) 1e+02 (Utilities|Array|MakeArray "ObjectTypeQuery1") "/Game/Building_Hider/Blueprints/BP_Building_Master.BP_Building_Master_C"))
              (if (> (Utilities|Array|Length _outactors) 0)
                (if (not (== (LocalVariables|GetNewBuildingLOCAL) (Utilities|Array|Get(acopy) _outactors)))
                  (Public|SetAutoHideMode false))))))))
    (:then_1
      (bind _output_get (Variables|Default|SetSelectedBuilding (LocalVariables|GetNewBuildingLOCAL)))
      (if (not (Variables|/Game/Building_Hider/Blueprints/BP_Building_Master.BP_Building_Master_C|GetBuildingActive (LocalVariables|GetNewBuildingLOCAL)))
        (Default|ActivateHidden _output_get)))
    (:then_2
      (Utilities|IsValid _buildingwidget
        (:Is%20Valid
          (Default|EventUpdateBuildingInfo _buildingwidget (Variables|Default|GetSelectedBuilding)))))))

(fn UnselectBuilding
  (Utilities|FlowControl|Sequence
    (:then_0
      (Utilities|IsValid (Variables|Default|GetSelectedBuilding)
        (:Is%20Valid
          (if (Variables|Default|GetAutoHide)
            (bind _outactors (Collision|SphereOverlapActors (Transformation|GetActorLocation (Pawn|GetControlledPawn (Game|GetPlayerController (Variables|Default|GetPlayerIndex)))) 1e+02 (Utilities|Array|MakeArray "ObjectTypeQuery1") "/Game/Building_Hider/Blueprints/BP_Building_Master.BP_Building_Master_C"))
            (if (> (Utilities|Array|Length _outactors) 0)
              (if (not (== (Variables|Default|GetSelectedBuilding) (Utilities|Array|Get(acopy) _outactors)))
                (Default|DeactivateHidden (Variables|Default|GetSelectedBuilding) false)
                (Variables|Default|SetSelectedBuilding 0))
              (else
                (Default|DeactivateHidden (Variables|Default|GetSelectedBuilding) false)
                (Variables|Default|SetSelectedBuilding 0)))
            (else
              (Default|DeactivateHidden (Variables|Default|GetSelectedBuilding) false)
              (Variables|Default|SetSelectedBuilding 0))))))
    (:then_1
      (Default|EventUpdateBuildingInfo (Variables|Default|GetBuildingWidget) (Variables|Default|GetSelectedBuilding)))))

(fn SetAutoHideMode
  (params (NewState :type Boolean))
  (bind _playerindex (Variables|Default|GetPlayerIndex))
  (bind _returnvalue (Game|GetPlayerController _playerindex))
  (bind _returnvalue_2 (Pawn|GetControlledPawn _returnvalue))
  (bind _returnvalue_3 (Transformation|GetActorLocation _returnvalue_2))
  (bind _output_get (Variables|Default|SetAutoHide NewState))
  (Default|SetAutoHideButtonState (Variables|Default|GetBuildingWidget) _output_get)
  (if _output_get
    (bind _outactors (Collision|SphereOverlapActors _returnvalue_3 1e+02 (Utilities|Array|MakeArray "ObjectTypeQuery1") "/Game/Building_Hider/Blueprints/BP_Building_Master.BP_Building_Master_C"))
    (if (> (Utilities|Array|Length _outactors) 0)
      (if (!= (Variables|Default|GetSelectedBuilding) (Utilities|Array|Get(acopy) _outactors))
        (Public|SelectBuilding (Utilities|Array|Get(acopy) _outactors))))
    (else
      (Utilities|IsValid (Variables|Default|GetSelectedBuilding)
        (:Is%20Not%20Valid
          (bind _outactors_2 (Collision|SphereOverlapActors _returnvalue_3 1e+02 (Utilities|Array|MakeArray "ObjectTypeQuery1") "/Game/Building_Hider/Blueprints/BP_Building_Master.BP_Building_Master_C"))
          (if (> (Utilities|Array|Length _outactors_2) 0)
            (bind _asbp_building_master (Utilities|Casting|CastToBP_Building_Master (Utilities|Array|Get(acopy) _outactors_2)))
            (Default|DeactivateHidden _asbp_building_master false)))))))

(fn SetPlayerFloorasActive
  (bind _selectedbuilding (Variables|Default|GetSelectedBuilding))
  (bind _playerindex (Variables|Default|GetPlayerIndex))
  (bind _returnvalue (Game|GetPlayerController _playerindex))
  (bind _returnvalue_2 (Pawn|GetControlledPawn _returnvalue))
  (bind _returnvalue_3 (Transformation|GetActorLocation _returnvalue_2))
  (Utilities|FlowControl|Sequence
    (:then_0
      (bind _outactors (Collision|SphereOverlapActors _returnvalue_3 1e+02 (Utilities|Array|MakeArray "ObjectTypeQuery1") "/Game/Building_Hider/Blueprints/BP_Building_Master.BP_Building_Master_C"))
      (if (> (Utilities|Array|Length _outactors) 0)
        (Public|SelectBuilding (Utilities|Array|Get(acopy) _outactors))))
    (:then_1
      (Utilities|IsValid _selectedbuilding
        (:Is%20Valid
          (Default|SwitchFloorto _selectedbuilding (Default|GetFloorbyLocation _selectedbuilding _returnvalue_3)))))))